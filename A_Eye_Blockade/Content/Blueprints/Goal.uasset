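; Goal actor that scores a point when the VR player reaches it and makes the course harder.
; When a VRPawn overlaps its Box, it moves the pawn to a fixed location and increments the Score stored on that pawn.
; The first and second points each spawn an Obstacle at a different hardcoded position, and later points spawn nothing more.
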(event OnComponentBeginOverlap(Box)
  (params (OverlappedComponent :type Primitive%20Component%20Object%20Reference) (OtherActor :type Actor%20Object%20Reference) (OtherComp :type Primitive%20Component%20Object%20Reference) (OtherBodyIndex :type Integer) (bFromSweep :type Boolean) (SweepResult :type Hit%20Result%20Structure%20%28by%20ref%29))
  (bind _asvrpawn (Utilities|Casting|CastToVRPawn OtherActor))
  (Transformation|SetActorLocation _asvrpawn "-1950.000000,240.000000,250.000000" false false)
  (Variables|/Game/VRTemplate/Blueprints/VRPawn.VRPawn_C|Setscore _asvrpawn (+ (Variables|/Game/VRTemplate/Blueprints/VRPawn.VRPawn_C|Getscore _asvrpawn) 1))
  (if (== (Variables|/Game/VRTemplate/Blueprints/VRPawn.VRPawn_C|Getscore _asvrpawn) 1)
    (Game|SpawnActorfromClass "/Game/Blueprints/Obstacle.Obstacle_C" (Math|Conversions|ToTransform(Vector) "-1180.000000,0.000000,0.000000") "Undefined" "MultiplyWithRoot" 0 0)
    (elif (== (Variables|/Game/VRTemplate/Blueprints/VRPawn.VRPawn_C|Getscore _asvrpawn) 2)
      (Game|SpawnActorfromClass "/Game/Blueprints/Obstacle.Obstacle_C" (Math|Conversions|ToTransform(Vector) "-260.000000,0.000000,0.000000") "Undefined" "MultiplyWithRoot" 0 0))))

(event EventBeginPlay)

(event Collision|EventActorBeginOverlap
  (params (OtherActor :type Actor%20Object%20Reference)))

(event EventTick
  (params (DeltaSeconds :type Float%20%28single-precision%29)))

(fn ConstructionScript)