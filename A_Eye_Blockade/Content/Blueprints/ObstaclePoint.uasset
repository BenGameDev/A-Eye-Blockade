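; ObstaclePoint handles exclusive path-point selection across three groups of three Point actor classes (1–3, 4–6, 7–9).
; Three check functions find each group's actors, disable PathPoint collision on the two losers of the first true flag, and print if none is true.
; A chained visibility-hiding version in the EventGraph is disconnected; BeginPlay only performs an unused Point2 lookup.
; Nothing in this Blueprint calls the check functions.
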(event EventBeginPlay
  (Actor|GetActorOfClass "/Game/Blueprints/point2.point2_C"))

(event EventTick
  (params (DeltaSeconds :type Float%20%28single-precision%29)))

(fn ConstructionScript)

(fn Path1to3Check
  (bind _returnvalue (Actor|GetActorOfClass "/Game/Blueprints/point1.point1_C"))
  (bind _returnvalue_2 (Actor|GetActorOfClass "/Game/Blueprints/point2.point2_C"))
  (bind _returnvalue_3 (Actor|GetActorOfClass "/Game/Blueprints/point3.point3_C"))
  (if (Variables|/Game/Blueprints/point1.point1_C|GetPoint1_0 _returnvalue)
    (Collision|SetCollisionEnabled (Variables|ObstaclePoint_C|GetPathPoint _returnvalue_2) "NoCollision")
    (elif (Variables|/Game/Blueprints/point2.point2_C|GetPoint2_0 _returnvalue_2)
      (Collision|SetCollisionEnabled (Variables|ObstaclePoint_C|GetPathPoint _returnvalue) "NoCollision")
      (elif (Variables|/Game/Blueprints/point3.point3_C|Getpoint3 _returnvalue_3)
        (Collision|SetCollisionEnabled (Variables|ObstaclePoint_C|GetPathPoint _returnvalue) "NoCollision")
        (else
          (Development|PrintString "No bool is true"))))))

(fn Path4to6Check
  (bind _returnvalue (Actor|GetActorOfClass "/Game/Blueprints/point4.point4_C"))
  (bind _returnvalue_2 (Actor|GetActorOfClass "/Game/Blueprints/point5.point5_C"))
  (bind _returnvalue_3 (Actor|GetActorOfClass "/Game/Blueprints/point6.point6_C"))
  (if (Variables|/Game/Blueprints/point4.point4_C|Getpoint4 _returnvalue)
    (Collision|SetCollisionEnabled (Variables|ObstaclePoint_C|GetPathPoint _returnvalue_2) "NoCollision")
    (elif (Variables|/Game/Blueprints/point5.point5_C|Getpoint5 _returnvalue_2)
      (Collision|SetCollisionEnabled (Variables|ObstaclePoint_C|GetPathPoint _returnvalue) "NoCollision")
      (elif (Variables|/Game/Blueprints/point6.point6_C|Getpoint6 _returnvalue_3)
        (Collision|SetCollisionEnabled (Variables|ObstaclePoint_C|GetPathPoint _returnvalue) "NoCollision")
        (else
          (Development|PrintString "No bool is true"))))))

(fn Path7to9Check
  (bind _returnvalue (Actor|GetActorOfClass "/Game/Blueprints/point7.point7_C"))
  (bind _returnvalue_2 (Actor|GetActorOfClass "/Game/Blueprints/point8.point8_C"))
  (bind _returnvalue_3 (Actor|GetActorOfClass "/Game/Blueprints/point9.point9_C"))
  (if (Variables|/Game/Blueprints/point7.point7_C|Getpoint7 _returnvalue)
    (Collision|SetCollisionEnabled (Variables|ObstaclePoint_C|GetPathPoint _returnvalue_2) "NoCollision")
    (elif (Variables|/Game/Blueprints/point8.point8_C|Getpoint8 _returnvalue_2)
      (Collision|SetCollisionEnabled (Variables|ObstaclePoint_C|GetPathPoint _returnvalue) "NoCollision")
      (elif (Variables|/Game/Blueprints/point9.point9_C|Getpoint9 _returnvalue_3)
        (Collision|SetCollisionEnabled (Variables|ObstaclePoint_C|GetPathPoint _returnvalue) "NoCollision")
        (else
          (Development|PrintString "No bool is true"))))))